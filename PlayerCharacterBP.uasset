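; PlayerCharacterBP provides grid-like movement events for a PlayerActor and shows a movement counter widget on screen at BeginPlay.
; Four custom events (Up, Down, Left, Right) each look up the first PlayerActor in the level and shift it a fixed step along world X or Y.
; Moves are instant teleports without sweep, so collision does not block them.
; The Blueprint moves that separate actor rather than itself and does not update the counter.
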(event `MovePlayerUp`
  (bind _outactors (`GameplayStatics.GetAllActorsOfClass` "/Game/Blueprints/PlayerActor.PlayerActor_C"))
  (bind _asplayer_actor (cast `/Game/Blueprints/PlayerActor` (`|GetArrayItem` _outactors)))
  (`self.K2_SetActorLocation` _asplayer_actor (`KismetMathLibrary.MakeVector` (+ (.x (`self.K2_GetActorLocation` _asplayer_actor)) 100.0) (.y (`self.K2_GetActorLocation` _asplayer_actor)) (.z (`self.K2_GetActorLocation` _asplayer_actor))) false true))

(event `MovePlayerDown`
  (bind _outactors (`GameplayStatics.GetAllActorsOfClass` "/Game/Blueprints/PlayerActor.PlayerActor_C"))
  (bind _asplayer_actor (cast `/Game/Blueprints/PlayerActor` (`|GetArrayItem` _outactors)))
  (`self.K2_SetActorLocation` _asplayer_actor (`KismetMathLibrary.MakeVector` (+ (.x (`self.K2_GetActorLocation` _asplayer_actor)) -100.0) (.y (`self.K2_GetActorLocation` _asplayer_actor)) (.z (`self.K2_GetActorLocation` _asplayer_actor))) false true))

(event `MovePlayerLeft`
  (bind _outactors (`GameplayStatics.GetAllActorsOfClass` "/Game/Blueprints/PlayerActor.PlayerActor_C"))
  (bind _asplayer_actor (cast `/Game/Blueprints/PlayerActor` (`|GetArrayItem` _outactors)))
  (`self.K2_SetActorLocation` _asplayer_actor (`KismetMathLibrary.MakeVector` (.x (`self.K2_GetActorLocation` _asplayer_actor)) (+ (.y (`self.K2_GetActorLocation` _asplayer_actor)) -100.0) (.z (`self.K2_GetActorLocation` _asplayer_actor))) false true))

(event `MovePlayerRight`
  (bind _outactors (`GameplayStatics.GetAllActorsOfClass` "/Game/Blueprints/PlayerActor.PlayerActor_C"))
  (bind _asplayer_actor (cast `/Game/Blueprints/PlayerActor` (`|GetArrayItem` _outactors)))
  (`self.K2_SetActorLocation` _asplayer_actor (`KismetMathLibrary.MakeVector` (.x (`self.K2_GetActorLocation` _asplayer_actor)) (+ (.y (`self.K2_GetActorLocation` _asplayer_actor)) 100.0) (.z (`self.K2_GetActorLocation` _asplayer_actor))) false true))

(event `self.ReceiveBeginPlay`
  (bind _returnvalue (`|CreateWidget` "/Game/Blueprints/MovementCounterWGT.MovementCounterWGT_C"))
  (`UserWidget.AddToViewport` _returnvalue 0))

(fn `UserConstructionScript`)